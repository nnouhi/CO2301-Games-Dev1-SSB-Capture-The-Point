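; BP_AICharacter is an enemy character that shows a health bar widget when the player is nearby.
; On BeginPlay it registers itself as the OwningActor of the WBP_EnemyHealthbar inside its Healthbar widget component.
; The MakeWidgetVisible collision component shows the bar when a BP_PlayerCharacter begins overlapping it and hides it when that overlap ends.
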(event OnComponentBeginOverlap(MakeWidgetVisible)
  (params (OverlappedComponent :type Primitive%20Component%20Object%20Reference) (OtherActor :type Actor%20Object%20Reference) (OtherComp :type Primitive%20Component%20Object%20Reference) (OtherBodyIndex :type Integer) (bFromSweep :type Boolean) (SweepResult :type Hit%20Result%20Structure%20%28by%20ref%29))
  (Utilities|Casting|CastToBP_PlayerCharacter OtherActor)
  (Rendering|SetVisibility (Variables|Default|GetHealthbar) true false))

(event OnComponentEndOverlap(MakeWidgetVisible)
  (params (OverlappedComponent :type Primitive%20Component%20Object%20Reference) (OtherActor :type Actor%20Object%20Reference) (OtherComp :type Primitive%20Component%20Object%20Reference) (OtherBodyIndex :type Integer))
  (Utilities|Casting|CastToBP_PlayerCharacter OtherActor)
  (Rendering|SetVisibility (Variables|Default|GetHealthbar) false false))

(event EventBeginPlay
  (bind _aswbp_enemy_healthbar (Utilities|Casting|CastToWBP_EnemyHealthbar (UserInterface|GetUserWidgetObject (Variables|Default|GetHealthbar))))
  (Variables|/Game/_Game/EnemyCharacter/Widgets/WBP_EnemyHealthbar.WBP_EnemyHealthbar_C|SetOwningActor _aswbp_enemy_healthbar self))

(event Collision|EventActorBeginOverlap
  (params (OtherActor :type Actor%20Object%20Reference)))

(event EventTick
  (params (DeltaSeconds :type Float%20%28single-precision%29)))

(fn ConstructionScript)